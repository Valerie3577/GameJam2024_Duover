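; BP_Snowpile is a snow pile zone that heals the player's snowman while it overlaps the box.
; BeginPlay caches the player BP_Snowman and the Variables game instance, where box overlaps toggle a shared InSnow flag.
; Begin overlap starts a short Delay loop that calls Heal while InSnow is set, or only prints a melting message if the snowman is lighted.
; Overlap events do not check which actor triggered them.
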(event OnComponentBeginOverlap(Box)
  (params (OverlappedComponent :type Primitive%20Component%20Object%20Reference) (OtherActor :type Actor%20Object%20Reference) (OtherComp :type Primitive%20Component%20Object%20Reference) (OtherBodyIndex :type Integer) (bFromSweep :type Boolean) (SweepResult :type Hit%20Result%20Structure%20%28by%20ref%29))
  (bind _variables (Variables|Default|GetVariables))
  (Variables|/Game/Blueprints/Variables.Variables_C|SetInSnow _variables true)
  (if (Variables|/Game/Blueprints/Variables.Variables_C|GetInSnow _variables) :!label _label
    (if (not (Variables|/Game/Blueprints/BP_Snowman.BP_Snowman_C|GetIsLighted (Variables|Default|GetSnowman)))
      (Utilities|FlowControl|Delay 0.1)
      (Default|Heal (Variables|Default|GetSnowman))
      (goto _label)
      (else
        (Development|PrintString "You're Melting")
        (Utilities|FlowControl|Delay 0.1)
        (goto _label)))
    (else
      (Development|PrintString "Not in Snow"))))

(event OnComponentEndOverlap(Box)
  (params (OverlappedComponent :type Primitive%20Component%20Object%20Reference) (OtherActor :type Actor%20Object%20Reference) (OtherComp :type Primitive%20Component%20Object%20Reference) (OtherBodyIndex :type Integer))
  (Variables|/Game/Blueprints/Variables.Variables_C|SetInSnow (Variables|Default|GetVariables) false))

(event EventBeginPlay
  (CallFunction|GetRefs))

(event Collision|EventActorBeginOverlap
  (params (OtherActor :type Actor%20Object%20Reference)))

(event EventTick
  (params (DeltaSeconds :type Float%20%28single-precision%29)))

(fn ConstructionScript)

(fn GetRefs
  (bind _asbp_snowman (Utilities|Casting|CastToBP_Snowman (Game|Player|GetPlayerPawn 0)))
  (Variables|Default|SetSnowman _asbp_snowman)
  (bind _asvariables (Utilities|Casting|CastToVariables (Game|GetGameInstance)))
  (Variables|Default|SetVariables _asvariables))