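; BP_Boulder is a boulder that is released when something enters its Trigger volume.
; BeginPlay casts the player character to BP_Snowman and caches it.
; Any overlap on Trigger enables physics simulation on the sphere component, without filtering the overlapping actor.
; The same event destroys the actor tagged "Destructible" that is nearest to the snowman, measured from the player's location rather than the boulder's.
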(event OnComponentBeginOverlap(Trigger)
  (params (OverlappedComponent :type Primitive%20Component%20Object%20Reference) (OtherActor :type Actor%20Object%20Reference) (OtherComp :type Primitive%20Component%20Object%20Reference) (OtherBodyIndex :type Integer) (bFromSweep :type Boolean) (SweepResult :type Hit%20Result%20Structure%20%28by%20ref%29))
  (Physics|SetSimulatePhysics (Variables|Default|GetSphere_BA84D302) true)
  (bind _outactors (Actor|GetAllActorswithTag "Destructible"))
  (Actor|DestroyActor (.ReturnValue (Actor|FindNearestActor (Transformation|GetActorLocation (Variables|Default|GetSnowman)) _outactors))))

(event EventBeginPlay
  (bind _asbp_snowman (Utilities|Casting|CastToBP_Snowman (Game|GetPlayerCharacter 0)))
  (Variables|Default|SetSnowman _asbp_snowman))

(event Collision|EventActorBeginOverlap
  (params (OtherActor :type Actor%20Object%20Reference)))

(event EventTick
  (params (DeltaSeconds :type Float%20%28single-precision%29)))

(fn ConstructionScript)