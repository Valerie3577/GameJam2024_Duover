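; Snowball projectile actor that destroys itself on overlapping a Floor-tagged actor and stops moving on any other overlap.
; The construction script applies its speed settings to ProjectileMovement, and BeginPlay copies the initial speed into the Variables game instance.
; IncreaseBallSpeed sets InitialSpeed to that stored value plus SpeedMultiplier, an additive offset despite its name.
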(event OnComponentBeginOverlap(Sphere1)
  (params (OverlappedComponent :type Primitive%20Component%20Object%20Reference) (OtherActor :type Actor%20Object%20Reference) (OtherComp :type Primitive%20Component%20Object%20Reference) (OtherBodyIndex :type Integer) (bFromSweep :type Boolean) (SweepResult :type Hit%20Result%20Structure%20%28by%20ref%29))
  (if (Actor|ActorHasTag OtherActor "Floor")
    (Development|PrintString "Floor")
    (Actor|DestroyActor)
    (else
      (Components|Movement|StopMovementImmediately (Variables|Default|GetProjectileMovement)))))

(event EventBeginPlay
  (bind _asvariables (Utilities|Casting|CastToVariables (Game|GetGameInstance)))
  (bind _output_get (Variables|Default|SetVariables _asvariables))
  (Variables|/Game/Blueprints/Variables.Variables_C|SetInitial%20Speed _output_get (Variables|/Script/Engine.ProjectileMovementComponent|GetInitialSpeed (Variables|Default|GetProjectileMovement))))

(event Collision|EventActorBeginOverlap
  (params (OtherActor :type Actor%20Object%20Reference)))

(event EventTick
  (params (DeltaSeconds :type Float%20%28single-precision%29)))

(fn ConstructionScript
  (bind _projectilemovement (Variables|Default|GetProjectileMovement))
  (Variables|/Script/Engine.ProjectileMovementComponent|SetInitialSpeed _projectilemovement (Variables|Default|GetSpeed))
  (Variables|/Script/Engine.ProjectileMovementComponent|SetMaxSpeed _projectilemovement (Variables|Default|GetMaxSpeed)))

(fn IncreaseBallSpeed
  (Variables|/Script/Engine.ProjectileMovementComponent|SetInitialSpeed (Variables|Default|GetProjectileMovement) (+ (Variables|/Game/Blueprints/Variables.Variables_C|GetInitial%20Speed (Variables|Default|GetVariables)) (Variables|Default|GetSpeedMultiplier))))